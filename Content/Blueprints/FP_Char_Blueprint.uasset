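; First-person player character for a photo-taking game with a monster, handling Enhanced Input movement, sprint, timeline-driven crouch and lean, and speed-based camera shakes.
; Camera mode toggles post-process volumes and spotlight, slows walking, and enables FOV zoom and render-target photo capture.
; A photo taken while a monster mesh is visible calls Noticed and starts a delayed falling-camera cutscene that fades in the photo widget.
; Jump and landing logic are disconnected.
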(event `EnhancedInput|/Game/Input/Crouch_IA`
  (params (ActionValue :type Boolean) (ElapsedSeconds :type "Float (double-precision)") (TriggeredSeconds :type "Float (double-precision)") (InputAction :type "InputAction Object Reference" :default "/Game/Input/Crouch_IA.Crouch_IA"))
  (bind _charactermovement (`self.CharacterMovement`))
  ;[1 1 1] Crouch (Held)
  (:`Triggered`
    (set `CharacterMovementComponent.MaxWalkSpeed` 300.0 _charactermovement)
    (bind (_direction _crouchalpha) (`Timeline|Crouch Timeline` :!label _label)
      (:`Update`
        (`CapsuleComponent.SetCapsuleHalfHeight` (`self.CapsuleComponent`) (`KismetMathLibrary.Lerp` 88.0 11.0 _crouchalpha) true))))
  (:`Completed`
    (set `CharacterMovementComponent.MaxWalkSpeed` 600.0 _charactermovement)
    (goto _label :!via `Reverse`)))

(event `EnhancedInput|/Game/Input/Sprint_IA`
  (params (ActionValue :type Boolean) (ElapsedSeconds :type "Float (double-precision)") (TriggeredSeconds :type "Float (double-precision)") (InputAction :type "InputAction Object Reference" :default "/Game/Input/Sprint_IA.Sprint_IA"))
  (bind _charactermovement (`self.CharacterMovement`))
  (bind _incamera (`self.inCamera`))
  ;[1 1 1] Simple Sprint
  (:`Triggered`
    (if (not _incamera)
      (set `CharacterMovementComponent.MaxWalkSpeed` 1300.0 _charactermovement)))
  (:`Completed`
    (if (not _incamera)
      (set `CharacterMovementComponent.MaxWalkSpeed` 600.0 _charactermovement))))

(event `self.ReceiveBeginPlay`
  ;[1 1 1] Add Input Controls
  (bind _asplayer_controller (cast `PlayerController` (`self.GetController`)))
  (bind _returnvalue (pcsubsystem `EnhancedInputLocalPlayerSubsystem` _asplayer_controller))
  (`/Engine/EditorBlueprintResources/StandardMacros.IsValid` _returnvalue
    (:`Is Valid`
      (`EnhancedInputSubsystemInterface.AddMappingContext` _returnvalue "/Game/Input/FP_InputMC.FP_InputMC" 0 (struct)))))

(event `EnhancedInput|/Game/Input/LeanLeft_IA`
  (params (ActionValue :type Boolean) (ElapsedSeconds :type "Float (double-precision)") (TriggeredSeconds :type "Float (double-precision)") (InputAction :type "InputAction Object Reference" :default "/Game/Input/LeanLeft_IA.LeanLeft_IA"))
  (bind _returnvalue (`GameplayStatics.GetPlayerController` 0))
  (bind _isrightlean (`self.isRightLean`))
  (bind _cameraspring (`self.CameraSpring`))
  (bind (_returnvalue_roll _returnvalue_pitch _returnvalue_yaw) (`KismetMathLibrary.BreakRotator` (`Controller.GetControlRotation` _returnvalue)))
  (bind (_relativelocation_x _relativelocation_y _relativelocation_z) (`KismetMathLibrary.BreakVector` (`SceneComponent.RelativeLocation` _cameraspring)))
  ;[1 1 1] Leaning
  (:`Triggered`
    (if (not _isrightlean)
      (bind (_direction _leanmation_left) (`Timeline|LeanLeft Timeline` :!label _label_2)
        (:`Update`
          (set `self.isLeftLean` true)
          (`SceneComponent.K2_SetRelativeLocation` _cameraspring (`KismetMathLibrary.MakeVector` _relativelocation_x (`KismetMathLibrary.Lerp` 0.0 (* (`self.Lean Location`) -1.0) _leanmation_left) _relativelocation_z) false false)
          (`Controller.SetControlRotation` _returnvalue (`KismetMathLibrary.MakeRotator` (* (* (`self.Lean Rotation`) -1.0) _leanmation_left) _returnvalue_pitch _returnvalue_yaw)))
        (:`Finished`
          (if (== (`TimelineComponent.GetPlaybackPosition` (`self.LeanRight Timeline`)) 0.0)
            (set `self.isLeftLean` false))))))
  (:`Completed`
    (if (not _isrightlean)
      (goto _label_2 :!via `Reverse`))))

(event `EnhancedInput|/Game/Input/Move_IA`
  (params (ActionValue :type "Vector2D Structure") (ElapsedSeconds :type "Float (double-precision)") (TriggeredSeconds :type "Float (double-precision)") (InputAction :type "InputAction Object Reference" :default "/Game/Input/Move_IA.Move_IA"))
  (:`Triggered`
    ;[1 1 1] Movement
    (if (not (`self.animPlaying`))
      (`self.AddMovementInput` (`self.GetActorRightVector`) ActionValue_X)
      (`self.AddMovementInput` (`self.GetActorForwardVector`) ActionValue_Y))))

(event `EnhancedInput|/Game/Input/LeanRight_IA`
  (params (ActionValue :type Boolean) (ElapsedSeconds :type "Float (double-precision)") (TriggeredSeconds :type "Float (double-precision)") (InputAction :type "InputAction Object Reference" :default "/Game/Input/LeanRight_IA.LeanRight_IA"))
  (bind _returnvalue (`GameplayStatics.GetPlayerController` 0))
  (bind _cameraspring (`self.CameraSpring`))
  (bind _isleftlean (`self.isLeftLean`))
  (bind (_returnvalue_roll _returnvalue_pitch _returnvalue_yaw) (`KismetMathLibrary.BreakRotator` (`Controller.GetControlRotation` _returnvalue)))
  (bind (_relativelocation_x _relativelocation_y _relativelocation_z) (`KismetMathLibrary.BreakVector` (`SceneComponent.RelativeLocation` _cameraspring)))
  ;[1 1 1] Leaning
  (:`Triggered`
    (if (not _isleftlean)
      (bind (_direction _leanmation_right) (`Timeline|LeanRight Timeline` :!label _label_3)
        (:`Update`
          (set `self.isRightLean` true)
          (`SceneComponent.K2_SetRelativeLocation` _cameraspring (`KismetMathLibrary.MakeVector` _relativelocation_x (`KismetMathLibrary.Lerp` 0.0 (`self.Lean Location`) _leanmation_right) _relativelocation_z) false false)
          (`Controller.SetControlRotation` _returnvalue (`KismetMathLibrary.MakeRotator` (* _leanmation_right (`self.Lean Rotation`)) _returnvalue_pitch _returnvalue_yaw)))
        (:`Finished`
          (if (== (`TimelineComponent.GetPlaybackPosition` (`self.LeanLeft Timeline`)) 0.0)
            (set `self.isRightLean` false))))))
  (:`Completed`
    (if (not _isleftlean)
      (goto _label_3 :!via `Reverse`))))

(event `EnhancedInput|/Game/Input/Look_IA`
  (params (ActionValue :type "Vector2D Structure") (ElapsedSeconds :type "Float (double-precision)") (TriggeredSeconds :type "Float (double-precision)") (InputAction :type "InputAction Object Reference" :default "/Game/Input/Look_IA.Look_IA"))
  (:`Triggered`
    ;[1 1 1] Look
    (if (not (`self.animPlaying`))
      (`self.AddControllerYawInput` (* ActionValue_X 0.7))
      (`self.AddControllerPitchInput` (* ActionValue_Y 0.7)))))

(event `EnhancedInput|/Game/Input/Jump_IA`
  (params (ActionValue :type Boolean) (ElapsedSeconds :type "Float (double-precision)") (TriggeredSeconds :type "Float (double-precision)") (InputAction :type "InputAction Object Reference" :default "/Game/Input/Jump_IA.Jump_IA"))
  ;[1 1 1] Jump (Deactivated and no negative camera pitch on land)
)

(event `self.ReceiveTick`
  (params (DeltaSeconds :type "Float (single-precision)"))
  (bind _returnvalue (`GameplayStatics.GetPlayerController` 0))
  (bind _returnvalue_2 (`KismetMathLibrary.VSize` (`self.GetVelocity`)))
  ;[1 1 1] Headshakes
  (if (and (> _returnvalue_2 0.0) (`self.CanJump`))
    (if (< _returnvalue_2 650.0)
      (`PlayerController.ClientStartCameraShake` :`self` _returnvalue :`Shake` "/Game/Blueprints/Effects/CameraShakeWalk.CameraShakeWalk_C")
      (else
        (`PlayerController.ClientStartCameraShake` :`self` _returnvalue :`Shake` "/Game/Blueprints/Effects/CameraShakeSprint.CameraShakeSprint_C")))
    (else
      (`PlayerController.ClientStartCameraShake` :`self` _returnvalue :`Shake` "/Game/Blueprints/Effects/CameraShakeIdle.CameraShakeIdle_C"))))

(event `self.OnLanded`
  (params (Hit :type "HitResult Structure (by ref)"))
  ;[1 1 1] Jump (Deactivated and no negative camera pitch on land)
)

(event `EnhancedInput|/Game/Input/Camera_IA`
  (params (ActionValue :type Boolean) (ElapsedSeconds :type "Float (double-precision)") (TriggeredSeconds :type "Float (double-precision)") (InputAction :type "InputAction Object Reference" :default "/Game/Input/Camera_IA.Camera_IA"))
  (bind _charactermovement (`self.CharacterMovement`))
  ;[1 1 1] Turn on Post Processing Effect and Set inCamera bool
  (:`Triggered`
    (`/Engine/EditorBlueprintResources/StandardMacros.DoOnce` false :!label _label_4
      (:`Completed`
        (bind _outactors (`GameplayStatics.GetAllActorsOfClass` "/Script/Engine.PostProcessVolume"))
        (if (`self.inCamera`)
          (for _array_element _outactors
            (set `PostProcessVolume.bEnabled` false _array_element)
            (set `self.inCamera` false)
            (`CameraComponent.SetFieldOfView` (`self.Camera`) 90.0)
            (set `self.Zoomed` false)
            (set `CharacterMovementComponent.MaxWalkSpeed` 600.0 _charactermovement)
            (`SceneComponent.ToggleVisibility` (`self.SpotLight`) false :!label _label_5)
            (`KismetSystemLibrary.Delay` 0.2)
            (goto _label_4 :!via `Reset`))
          (else
            (for _array_element_2 _outactors
              (set `PostProcessVolume.bEnabled` true _array_element_2)
              (set `self.inCamera` true)
              (set `CharacterMovementComponent.MaxWalkSpeed` 150.0 _charactermovement)
              (goto _label_5))))))))

(event `EnhancedInput|/Game/Input/TakePhoto_IA`
  (params (ActionValue :type Boolean) (ElapsedSeconds :type "Float (double-precision)") (TriggeredSeconds :type "Float (double-precision)") (InputAction :type "InputAction Object Reference" :default "/Game/Input/TakePhoto_IA.TakePhoto_IA"))
  (bind _scenecapturecomponent2d (`self.SceneCaptureComponent2D`))
  ;[1 1 1] Take Photo and Save to TakenPhotos Folder
  (:`Triggered`
    (if (`self.inCamera`)
      (`/Engine/EditorBlueprintResources/StandardMacros.DoOnce` false :!label _label_6
        (:`Completed`
          (bind _returnvalue (`KismetRenderingLibrary.CreateRenderTarget2D` 400 230))
          (`SceneCaptureComponent2D.CaptureScene` _scenecapturecomponent2d)
          (bind _output_get (set `SceneCaptureComponent2D.TextureTarget` _returnvalue _scenecapturecomponent2d))
          (bind _outactors (`GameplayStatics.GetAllActorsOfClass` "/Game/Blueprints/Monster_Blueprint.Monster_Blueprint_C"))
          (for _array_element _outactors
            (if (`SceneComponent.IsVisible` (`Character.Mesh` _array_element))
              (set `self.phototaken` true)
              (`/Game/Blueprints/Monster_Blueprint.noticed` _array_element)
              (`self.cutscene`))
            (`KismetSystemLibrary.Delay` 0.2)
            (goto _label_6 :!via `Reset`)))))))

(event `EnhancedInput|/Game/Input/ZoomIn_IA`
  (params (ActionValue :type Boolean) (ElapsedSeconds :type "Float (double-precision)") (TriggeredSeconds :type "Float (double-precision)") (InputAction :type "InputAction Object Reference" :default "/Game/Input/ZoomIn_IA.ZoomIn_IA"))
  ;[1 1 1] Zoom for Camera Mode
  (:`Triggered`
    (if (`self.inCamera`)
      (if (not (`self.Zoomed`))
        (set `self.Zoomed` true)
        (bind (_direction _newtrack_0) (`Timeline|FOV Timeline` :!label _label_7)
          (:`Update`
            (`CameraComponent.SetFieldOfView` (`self.Camera`) _newtrack_0)))))))

(event `EnhancedInput|/Game/Input/ZoomOut_IA`
  (params (ActionValue :type Boolean) (ElapsedSeconds :type "Float (double-precision)") (TriggeredSeconds :type "Float (double-precision)") (InputAction :type "InputAction Object Reference" :default "/Game/Input/ZoomOut_IA.ZoomOut_IA"))
  ;[1 1 1] Zoom for Camera Mode
  (:`Triggered`
    (if (`self.inCamera`)
      (if (`self.Zoomed`)
        (set `self.Zoomed` false)
        (goto _label_7 :!via `Reverse`)))))

(event `cutscene`
  (bind _returnvalue (`GameplayStatics.GetPlayerController` 0))
  (bind _returnvalue_2 (`GameplayStatics.GetPlayerController` 0))
  (bind _cameraspring (`self.CameraSpring`))
  (bind (_returnvalue_roll _returnvalue_pitch _returnvalue_yaw) (`KismetMathLibrary.BreakRotator` (`Controller.GetControlRotation` _returnvalue)))
  (bind (_returnvalue_roll_2 _returnvalue_pitch_2 _returnvalue_yaw_2) (`KismetMathLibrary.BreakRotator` (`Controller.GetControlRotation` _returnvalue_2)))
  (bind (_relativelocation_x _relativelocation_y _relativelocation_z) (`KismetMathLibrary.BreakVector` (`SceneComponent.RelativeLocation` _cameraspring)))
  ;[1 1 1] Cutscene
  (`KismetSystemLibrary.Delay` 15.0)
  (set `self.animPlaying` true)
  (bind (_direction _sighs _fall) (`Timeline|Cutscene Timeline`)
    (:`Update`
      (`Controller.SetControlRotation` _returnvalue_2 (`KismetMathLibrary.MakeRotator` _returnvalue_roll_2 _sighs _returnvalue_yaw_2))
      (`SceneComponent.K2_SetRelativeLocation` _cameraspring (`KismetMathLibrary.MakeVector` _relativelocation_x (/ _fall 10.0) _relativelocation_z) false false)
      (`Controller.SetControlRotation` _returnvalue (`KismetMathLibrary.MakeRotator` _fall _returnvalue_pitch _returnvalue_yaw))
      (`KismetSystemLibrary.Delay` 7.0)
      (bind _returnvalue_3 (`|CreateWidget` "/Game/Blueprints/NewWidgetBlueprint.NewWidgetBlueprint_C" null (stale `EnhancedInput|/Game/Input/TakePhoto_IA` _output_get)))
      (`UserWidget.AddToViewport` _returnvalue_3 0)
      (`UserWidget.PlayAnimation` _returnvalue_3 (`/Game/Blueprints/NewWidgetBlueprint.fadein` _returnvalue_3) 0.0 1 "Forward" 1.0 false))))

(event `EnhancedInput|/Game/Input/animTest_IA`
  (params (ActionValue :type Boolean) (ElapsedSeconds :type "Float (double-precision)") (TriggeredSeconds :type "Float (double-precision)") (InputAction :type "InputAction Object Reference" :default "/Game/Input/animTest_IA.animTest_IA"))
  ;[1 1 1] Cutscene
)

(fn `UserConstructionScript`)